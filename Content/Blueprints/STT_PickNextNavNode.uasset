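; StateTree task that picks the next NavNode in a chain of linked navigation nodes.
; On state entry with no valid CurrentNode, it seeds one from the first NavNode in the level and requests a random next node, passing in PreviousNode.
; A valid result shifts Current to Previous and finishes successfully, otherwise it fails.
; An already valid CurrentNode triggers no logic, leaving the task unfinished.
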(event EventLatentEnterState
  (params (Transition :type State%20Tree%20Transition%20Result%20Structure%20%28by%20ref%29))
  (Variables|Default|GetCurrentNode
    (:then)
    (:else
      (bind _outactors (Actor|GetAllActorsOfClass "/Script/EchoesOfTime.NavNode"))
      (bind _output_get (Variables|Default|SetCurrentNode (Utilities|Array|Get(acopy) _outactors)))
      (bind _output_get_2 (Variables|Default|SetNextNode (Class|NavNode|GetRandomNextNode _output_get (Variables|Default|GetPreviousNode))))
      (Utilities|IsValid _output_get_2
        (:Is%20Valid
          (Variables|Default|SetPreviousNode (Variables|Default|GetCurrentNode))
          (Variables|Default|SetCurrentNode (Variables|Default|GetNextNode))
          (StateTree|FinishTask true))
        (:Is%20Not%20Valid
          (StateTree|FinishTask false))))))