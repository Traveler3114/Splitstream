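; StateTree task that makes an AI pawn wander between linked NavNode actors.
; On entering the state, it sets the current node to the first NavNode found in the world and asks it for a random next node, passing in the previous one.
; AIMoveTo sends the pawn there; success shifts the node references and finishes the task successfully, while failure finishes it as failed.
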(event EventLatentEnterState
  (params (Transition :type State%20Tree%20Transition%20Result%20Structure%20%28by%20ref%29))
  (bind _outactors (Actor|GetAllActorsOfClass "/Script/EchoesOfTime.NavNode"))
  (bind _output_get (Variables|Default|SetCurrentNode (Utilities|Array|Get(acopy) _outactors)))
  (Variables|Default|SetNextNode (Class|NavNode|GetRandomNextNode _output_get (Variables|Default|GetPreviousNode)))
  (AI|AIMoveTo (Variables|Default|GetPawn) "0, 0, 0" (Variables|Default|GetNextNode) 5.0 false
    (:OnSuccess
      (Variables|Default|SetPreviousNode (Variables|Default|GetCurrentNode))
      (Variables|Default|SetCurrentNode (Variables|Default|GetNextNode))
      (Variables|Default|SetNextNode 0)
      (StateTree|FinishTask true))
    (:OnFail
      (StateTree|FinishTask false))))