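; Default player controller that shows a win screen when collected money reaches its target and provides a toggle for detection immunity.
; Tab or Tilde flip-flops applying GE_DetectionImmunity to the controlled pawn's Ability System Component and removing it through the stored handle.
; On remote instances, Tick prints a debug string while the pawn has the Character.Status.Immunity tag.
; The money-changed event calls its parent, then creates WBP_WinScreen once Current equals Target.
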(event Custom|GameplayEffect
  (bind _returnvalue (Pawn|GetControlledPawn))
  (bind _returnvalue_2 (Ability|GetAbilitySystemComponent _returnvalue))
  (Utilities|FlowControl|FlipFlop
    (:A
      (bind _returnvalue_3 (GameplayEffects|ApplyGameplayEffectToSelf :self _returnvalue_2 :GameplayEffectClass "/Game/Blueprints/AbilitySystem/GameplayEffects/GE_DetectionImmunity.GE_DetectionImmunity_C"))
      (Variables|Default|SetActiveGameplayEffect _returnvalue_3))
    (:B
      (GameplayEffects|RemoveActiveGameplayEffect _returnvalue_2 (Variables|Default|GetActiveGameplayEffect) -1))))

(event EventOnMoneyCollectedChanged
  (params (Current :type Integer) (Target :type Integer))
  (|CallParentFunction Current Target)
  (if (== Current Target)
    (bind _returnvalue (UserInterface|CreateWidget "/Game/Blueprints/Widgets/WBP_WinScreen.WBP_WinScreen_C" self))
    (UserInterface|Viewport|AddtoViewport _returnvalue 0)))

(event EventTick
  (params (DeltaSeconds :type Float%20%28single-precision%29))
  (bind _returnvalue (Pawn|GetControlledPawn))
  (bind _returnvalue_2 (Ability|GetAbilitySystemComponent _returnvalue))
  (Networking|SwitchHasAuthority
    (:Remote
      (Utilities|IsValid _returnvalue_2
        (:Is%20Valid
          (if (GameplayTags|HasMatchingGameplayTag _returnvalue_2 "(TagName=\"Character.Status.Immunity\")")
            (Development|PrintString "Character.Status.Immunity")))))))

(event Input|KeyboardEvents|Tab
  (params (Key :type Key%20Structure :default "None"))
  (:Pressed
    (CallFunction|GameplayEffect)))

(event Input|KeyboardEvents|Tilde
  (params (Key :type Key%20Structure :default "None"))
  (:Pressed
    (CallFunction|GameplayEffect)))

(fn ConstructionScript)