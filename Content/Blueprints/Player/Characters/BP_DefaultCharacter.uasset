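; BP_DefaultCharacter is a player character Blueprint that switches its camera between aiming and normal look views.
; StartAimCamera and StopAimCamera re-attach the Camera to the CameraAim or CameraLook socket on the Mesh, keeping relative transforms.
; An AimTimeline that would interpolate camera location and rotation is left unconnected and never runs.
; IsActorAlreadyDetected is a stub that always returns false.
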(event EventStartAimCamera
  (params (AimLocation :type Vector :default "0, 0, 0") (AimRotation :type Rotator :default "0, 0, 0"))
  (Transformation|AttachComponentToComponent (Variables|Default|GetCamera) (Variables|Character|GetMesh) "CameraAim" "KeepRelative" "KeepRelative" "KeepRelative" true))

(event EventStopAimCamera
  (params (ReturnLocation :type Vector :default "0, 0, 0") (ReturnRotation :type Rotator :default "0, 0, 0"))
  (Transformation|AttachComponentToComponent (Variables|Default|GetCamera) (Variables|Character|GetMesh) "CameraLook" "KeepRelative" "KeepRelative" "KeepRelative" true))

(fn ConstructionScript)

(fn IsActorAlreadyDetected
  (params (DetectingActor :type Actor%20Object%20Reference))
  (return false))