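; BP_SafeDepositBoxSmall is a small lootable safe deposit box that opens when its lock is picked.
; Interact and cancel calls forward to LockPickComp, and no item is required.
; On unlock, timelines yaw the cover open and slide the box out, with each cover update restarting the box timeline.
; Custom depth highlights the cover and box only while locked.
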(event OnUnlock(LockPickComp)
  (bind _coverfloat (Timeline|CoverTL PlayFromStart)
    (:Update
      (Transformation|SetRelativeRotation (Variables|Default|GetCover) (Math|Rotator|MakeRotator 0.0 0.0 (Math|Float|Lerp 0.0 -9e+01 _coverfloat)) false false)
      (bind _depositboxfloat (Timeline|DepositBoxTL PlayFromStart)
        (:Update
          (Transformation|SetRelativeLocation (Variables|Default|GetDepositBox) (Math|Vector|MakeVector 0.0 (Math|Float|Lerp 0.0 6e+01 _depositboxfloat) 0.0) false false))))))

(event EventInteract
  (params (Interactor :type Actor%20Object%20Reference))
  (bind _lockpickcomp (Variables|Default|GetLockPickComp)
    (:then
      (Class|LockPickComponent|Interact _lockpickcomp Interactor))
    (:else)))

(event EventSetHighlighted
  (params (bHighlight :type Boolean))
  (if (not (Variables|/Script/EchoesOfTime.LockPickComponent|GetbUnlocked (Variables|Default|GetLockPickComp)))
    (Rendering|SetRenderCustomDepth (Variables|Default|GetCover) bHighlight)
    (Rendering|SetRenderCustomDepth (Variables|Default|GetDepositBox) bHighlight)
    (Rendering|SetRenderCustomDepth (Variables|Default|GetCover) bHighlight)
    (Rendering|SetRenderCustomDepth (Variables|Default|GetDepositBox) bHighlight)
    (else
      (Rendering|SetRenderCustomDepth (Variables|Default|GetCover) false)
      (Rendering|SetRenderCustomDepth (Variables|Default|GetDepositBox) false)
      (Rendering|SetRenderCustomDepth (Variables|Default|GetCover) false)
      (Rendering|SetRenderCustomDepth (Variables|Default|GetDepositBox) false))))

(event EventCancelInteract
  (params (Interactor :type Actor%20Object%20Reference))
  (Class|LockPickComponent|CancelInteract (Variables|Default|GetLockPickComp) Interactor))

(fn ConstructionScript)

(fn IsCorrectItem
  (params (Item :type Item%20Base%20Object%20Reference))
  (return false))

(fn IsProgressiveInteract
  (return false))

(fn RequiresItem
  (return false))