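; BP_Jewelry1 is a lootable jewelry actor that adds a random amount of collected money to DefaultGameState when interacted with, then destroys itself.
; The construction script gives JewelryMesh a random mesh from the Meshes array.
; Highlighting toggles custom depth and its stencil value on the mesh.
; The interaction query functions all return false, so looting is non-progressive and requires no item.
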(event EventInteract
  (params (Interactor :type Actor%20Object%20Reference))
  (bind _asdefault_game_state (Utilities|Casting|CastToDefaultGameState (Game|GetGameState)))
  (Class|DefaultGameState|AddCollectedMoney _asdefault_game_state (Math|Random|RandomIntegerinRange 100 500))
  (Actor|DestroyActor))

(event EventSetHighlighted
  (params (bHighlight :type Boolean))
  (bind _jewelrymesh (Variables|Default|GetJewelryMesh))
  (Rendering|SetRenderCustomDepth _jewelrymesh bHighlight)
  (Rendering|SetCustomDepthStencilValue _jewelrymesh (Math|Conversions|ToInteger(Boolean) bHighlight)))

(fn ConstructionScript
  (bind _meshes (Variables|Default|GetMeshes))
  (Components|StaticMesh|SetStaticMesh (Variables|Default|GetJewelryMesh) (Utilities|Array|Get(acopy) _meshes (Math|Random|RandomIntegerinRange 0 (- (Utilities|Array|Length _meshes) 1)))))

(fn IsCorrectItem
  (params (Item :type Item%20Base%20Object%20Reference))
  (return false))

(fn IsProgressiveInteract
  (return false))

(fn RequiresItem
  (return false))