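; BP_DisplayCase is a lockpickable display case actor that players interact with progressively, without needing an item.
; It forwards interact and cancel calls to its LockPick component and listens for that component's unlock event.
; On unlock, it hides the glass and disables its collision.
; Highlighting uses custom depth and stencil on the case mesh and is turned off once the lock is open.
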(event Custom|OnUnlock
  (bind _displaycaseglass (Variables|Default|GetDisplayCaseGlass))
  (Class|Interactable|SetHighlighted false)
  (Variables|/Script/EchoesOfTime.LockPickComponent|SetbUnlocked (Variables|Default|GetLockPick) true)
  (Rendering|SetVisibility _displaycaseglass false false)
  (Collision|SetCollisionEnabled _displaycaseglass "NoCollision"))

(event EventInteract
  (params (Interactor :type Actor%20Object%20Reference))
  (Class|LockPickComponent|Interact (Variables|Default|GetLockPick) Interactor))

(event EventCancelInteract
  (params (Interactor :type Actor%20Object%20Reference))
  (Class|LockPickComponent|CancelInteract (Variables|Default|GetLockPick) Interactor))

(event EventBeginPlay
  (EventDispatchers|BindEventtoOnUnlock (Variables|Default|GetLockPick) (delegate Custom|OnUnlock)))

(event EventSetHighlighted
  (params (bHighlight :type Boolean))
  (bind _displaycase (Variables|Default|GetDisplayCase))
  (if (Variables|/Script/EchoesOfTime.LockPickComponent|GetbUnlocked (Variables|Default|GetLockPick))
    (Rendering|SetRenderCustomDepth _displaycase false)
    (Rendering|SetCustomDepthStencilValue _displaycase 0)
    (else
      (Rendering|SetRenderCustomDepth (Variables|Default|GetDisplayCase) bHighlight)
      (Rendering|SetCustomDepthStencilValue (Variables|Default|GetDisplayCase) (Math|Conversions|ToInteger(Boolean) bHighlight)))))

(fn ConstructionScript)

(fn IsCorrectItem
  (params (Item :type Item%20Base%20Object%20Reference))
  (return false))

(fn IsProgressiveInteract
  (return true))

(fn RequiresItem
  (return false))