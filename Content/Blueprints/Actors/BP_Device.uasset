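; BP_Device is an interactable actor that launches the firewall minigame when used.
; Highlighting toggles custom depth rendering on its static mesh.
; Interact constructs a BP_FirerwallMiniGame object and starts it with the interactor's player controller.
; It reports that it needs no item, accepts none, and is not a progressive interaction.
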(event EventSetHighlighted
  (params (bHighlight :type Boolean))
  (Rendering|SetRenderCustomDepth (Variables|Default|GetStaticMesh) bHighlight))

(event EventInteract
  (params (Interactor :type Actor%20Object%20Reference))
  (bind _returnvalue (Game|ConstructObjectfromClass "/Game/Blueprints/Minigames/BP_FirerwallMiniGame.BP_FirerwallMiniGame_C"))
  (Class|FirewallMiniGame|StartGame _returnvalue (.AsPlayer%20Controller (Utilities|Casting|CastToPlayerController (Game|GetInstigatorController Interactor)))))

(fn ConstructionScript)

(fn IsCorrectItem
  (params (Item :type Item%20Base%20Object%20Reference))
  (return false))

(fn IsProgressiveInteract
  (return false))

(fn RequiresItem
  (return false))