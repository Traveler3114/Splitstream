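; Ghost actor that shows a mirrored copy of a referenced character at a fixed world-space offset.
; On begin play it copies the character's skeletal mesh, follows its pose through a leader pose component and applies a cloth material to two material slots.
; Each tick it matches the character's rotation and position, shifted far along Y and slightly down in Z.
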(event EventBeginPlay
  (bind _charactertomirror (Variables|Default|GetCharacterToMirror))
  (bind _ghostmesh (Variables|Default|GetGhostMesh))
  (bind _mesh (Variables|/Script/Engine.Character|GetMesh _charactertomirror))
  (Components|SkeletalMesh|SetSkeletalMeshAsset (Variables|Default|GetGhostMesh) (Components|SkeletalMesh|GetSkeletalMeshAsset _mesh))
  (Components|SkinnedMesh|SetLeaderPoseComponent (Variables|Default|GetGhostMesh) _mesh true true)
  (Rendering|Material|SetMaterial _ghostmesh 0 "/Engine/EngineDebugMaterials/ClothMaterial_WF.ClothMaterial_WF")
  (Rendering|Material|SetMaterial _ghostmesh 1 "/Engine/EngineDebugMaterials/ClothMaterial_WF.ClothMaterial_WF"))

(event EventTick
  (params (DeltaSeconds :type Float%20%28single-precision%29))
  (bind _charactertomirror (Variables|Default|GetCharacterToMirror))
  (bind _returnvalue (Transformation|GetActorLocation _charactertomirror))
  (Transformation|SetActorLocation (Math|Vector|MakeVector (.x _returnvalue) (- (.y _returnvalue) 4.91e+03) (- (.z _returnvalue) 8e+01)) false false)
  (Transformation|SetActorRotation (Transformation|GetActorRotation _charactertomirror)))

(fn ConstructionScript)