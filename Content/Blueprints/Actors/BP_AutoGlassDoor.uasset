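; BP_AutoGlassDoor is an automatic double glass door that opens for any Pawn entering its trigger box.
; Box overlap plays a Timeline, and end overlap reverses it, so the panes slide back when a Pawn leaves.
; The Timeline's DoorFloat track lerps the relative offset of GlassLeft along X and GlassRight along Y.
; It does not count occupants, so any Pawn leaving starts closing the door.
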(event OnComponentBeginOverlap(Box)
  (params (OverlappedComponent :type Primitive%20Component%20Object%20Reference) (OtherActor :type Actor%20Object%20Reference) (OtherComp :type Primitive%20Component%20Object%20Reference) (OtherBodyIndex :type Integer) (bFromSweep :type Boolean) (SweepResult :type Hit%20Result%20Structure%20%28by%20ref%29))
  (bind _glassleft (Variables|Default|GetGlassLeft))
  (bind _glassright (Variables|Default|GetGlassRight))
  (bind _relativelocation (Variables|/Script/Engine.SceneComponent|GetRelativeLocation _glassright))
  (bind _relativelocation_2 (Variables|/Script/Engine.SceneComponent|GetRelativeLocation _glassleft))
  (Utilities|Casting|CastToPawn OtherActor)
  (bind _doorfloat (Timeline|Timeline Play)
    (:Update
      (Transformation|SetRelativeLocation _glassleft (Math|Vector|MakeVector (Math|Float|Lerp 0.0 2e+02 _doorfloat) (.y _relativelocation_2) (.z _relativelocation_2)) false false)
      (Transformation|SetRelativeLocation _glassright (Math|Vector|MakeVector (.x _relativelocation) (Math|Float|Lerp 0.0 2e+02 _doorfloat) (.z _relativelocation)) false false))))

(event OnComponentEndOverlap(Box)
  (params (OverlappedComponent :type Primitive%20Component%20Object%20Reference) (OtherActor :type Actor%20Object%20Reference) (OtherComp :type Primitive%20Component%20Object%20Reference) (OtherBodyIndex :type Integer))
  (bind _glassleft (Variables|Default|GetGlassLeft))
  (bind _glassright (Variables|Default|GetGlassRight))
  (bind _relativelocation (Variables|/Script/Engine.SceneComponent|GetRelativeLocation _glassright))
  (bind _relativelocation_2 (Variables|/Script/Engine.SceneComponent|GetRelativeLocation _glassleft))
  (Utilities|Casting|CastToPawn OtherActor)
  (bind _doorfloat (Timeline|Timeline Reverse)
    (:Update
      (Transformation|SetRelativeLocation _glassleft (Math|Vector|MakeVector (Math|Float|Lerp 0.0 2e+02 _doorfloat) (.y _relativelocation_2) (.z _relativelocation_2)) false false)
      (Transformation|SetRelativeLocation _glassright (Math|Vector|MakeVector (.x _relativelocation) (Math|Float|Lerp 0.0 2e+02 _doorfloat) (.z _relativelocation)) false false))))

(fn ConstructionScript)