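; Default player state Blueprint that holds a team name and fetches the player's Steam avatar.
; BeginPlay forces the player state at index 1 onto the Future team, a testing shortcut noted as unnecessary in packaged builds.
; RequestAvatar looks up the medium Steam avatar by unique net ID and applies it on success.
; Disconnected debug nodes print team and illegal-status gameplay tags from the ability system component.
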(event EventTick
  (params (DeltaSeconds :type Float%20%28single-precision%29)))

(event EventRequestAvatar
  (bind _returnvalue (Class|AdvancedSteamFriendsLibrary|GetSteamFriendAvatar (Class|AdvancedSessionsLibrary|GetUniqueNetIDfromPlayerState self) "SteamAvatar_Medium")
    (:OnSuccess
      (Class|DefaultPlayerState|SetAvatarTexture _returnvalue))))

(event EventBeginPlay
  ;[0.15 0.15 0.15 0.5] So second player is always on future team, unnecessary in the packaged game
  (bind _asbp_default_player_state (Utilities|Casting|CastToBP_DefaultPlayerState (Game|GetPlayerState 1)))
  (Variables|/Script/EchoesOfTime.DefaultPlayerState|SetTeamName _asbp_default_player_state "Future"))

(fn ConstructionScript)